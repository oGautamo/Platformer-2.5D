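; BP_CameraManager is an actor that smoothly trails a follow target as a camera manager.
; Each tick, UpdateCameraPos interpolates its location with VInterpTo toward the target's position plus the target's forward vector and a camera offset.
; When LockCamera is set, the base height comes from the manager's current Z instead of the target's.
; Only location is updated; rotation is untouched.
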(event `self.ReceiveTick`
  (params (DeltaSeconds :type "Float (single-precision)"))
  (`self.UpdateCameraPos`))

(fn `UpdateCameraPos`
  (bind (_returnvalue_x _returnvalue_y _returnvalue_z) (`KismetMathLibrary.BreakVector` (`self.K2_GetActorLocation`)))
  (bind (_returnvalue_x_2 _returnvalue_y_2 _returnvalue_z_2) (`KismetMathLibrary.BreakVector` (`self.K2_GetActorLocation` (`self.FollowTarget`))))
  (`self.K2_SetActorLocation` (`KismetMathLibrary.VInterpTo` (`self.K2_GetActorLocation`) (+ (`KismetMathLibrary.MakeVector` _returnvalue_x_2 _returnvalue_y_2 (select `bool` (`self.LockCamera`) :`false` _returnvalue_z_2 :`true` _returnvalue_z)) (+ (`self.GetActorForwardVector` (`self.FollowTarget`)) (`self.Cam Offset`))) (`GameplayStatics.GetWorldDeltaSeconds`) (`self.Interp Speed`))))

(fn `UserConstructionScript`)